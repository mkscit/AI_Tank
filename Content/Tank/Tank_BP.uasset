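; Tank Blueprint that drives and turns its Body component from either player input or AI commands.
; Player input axes and custom AI events each apply frame-time-scaled local movement along X and yaw rotation directly to Body.
; The AI events mirror the player controls but use much lower move and turn rates.
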(event `InputAxis|MoveForwardBackward`
  (params (AxisValue :type "Float (single-precision)"))
  ;[1 1 1] Move Forward BackWard
  (`SceneComponent.K2_AddLocalTransform` (`self.Body`) (`KismetMathLibrary.MakeTransform` (* (* (2000.0 0.0 0.0) AxisValue) (`GameplayStatics.GetWorldDeltaSeconds`))) false false))

(event `self.AIMoveForward`
  (params (Axis :type "Float (single-precision)"))
  ;[1 1 1] Move Forward BackWard
  (`SceneComponent.K2_AddLocalTransform` (`self.Body`) (`KismetMathLibrary.MakeTransform` (* (* (250.0 0.0 0.0) Axis) (`GameplayStatics.GetWorldDeltaSeconds`))) false false))

(event `InputAxis|TurnLeftRight`
  (params (AxisValue :type "Float (single-precision)"))
  (`SceneComponent.K2_AddLocalRotation` (`self.Body`) (`KismetMathLibrary.MakeRotator` 0.0 0.0 (* 40.0 AxisValue (`GameplayStatics.GetWorldDeltaSeconds`))) false false))

(event `self.AITurnLR`
  (params (Axis :type "Float (single-precision)"))
  (`SceneComponent.K2_AddLocalRotation` (`self.Body`) (`KismetMathLibrary.MakeRotator` 0.0 0.0 (* 1.0 Axis (`GameplayStatics.GetWorldDeltaSeconds`))) false false))

(fn `UserConstructionScript`)